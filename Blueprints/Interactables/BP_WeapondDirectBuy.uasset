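; Interactable ammo purchase point for one weapon, chosen by WeaponIndex, that reports a fixed price and ammo type as its interaction details.
; The weapon's data table row selects the ammo sprite on begin play, which yaws toward the camera every tick.
; On interact, it compares an ability system attribute to that weapon's ammo maximum and, if below, calls the player's WeaponPickup and plays a buy sound, without deducting money itself.
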(event `self.ReceiveBeginPlay`
  (bind _ammo_sprite (`self.Ammo Sprite`))
  (bind _returnvalue (`|GetDataTableRow` "/Game/DirtyManners/Blueprints/Weapons/DT_DirtyMannersWeapons.DT_DirtyMannersWeapons" (`KismetStringLibrary.Conv_StringToName` (`KismetStringLibrary.Conv_IntToString` (`self.Weapon Index`))))
    (:`then`
      (switch `/Game/DirtyManners/Blueprints/Enums/ENUM_WeaponList` (`.WeaponName_2_ED9A753648A3CF613FAE83B21A06C6AA` (break `/Game/DirtyManners/Blueprints/Structs/ST_WeaponData` _returnvalue))
        (:`NewEnumerator2`
          (`PaperSpriteComponent.SetSprite` _ammo_sprite null))
        (:`NewEnumerator0`
          (`PaperSpriteComponent.SetSprite` _ammo_sprite "/Game/DirtyManners/Textures/UI/water_Sprite.water_Sprite"))
        (:`NewEnumerator1`
          (`PaperSpriteComponent.SetSprite` _ammo_sprite "/Game/DirtyManners/Textures/UI/WaterBalloon_Sprite.WaterBalloon_Sprite"))
        (:`NewEnumerator3`
          (`PaperSpriteComponent.SetSprite` _ammo_sprite "/Game/DirtyManners/Textures/UI/soap_resized_Sprite.soap_resized_Sprite"))))))

(event `self.ReceiveTick`
  (params (DeltaSeconds :type "Float (single-precision)"))
  (bind _returnvalue (`GameplayStatics.GetPlayerCameraManager` 0))
  (bind _ammo_sprite (`self.Ammo Sprite`))
  (bind (_returnvalue_roll _returnvalue_pitch _returnvalue_yaw) (`KismetMathLibrary.BreakRotator` (`KismetMathLibrary.FindLookAtRotation` (`SceneComponent.K2_GetComponentLocation` _ammo_sprite) (`PlayerCameraManager.GetCameraLocation` _returnvalue))))
  (`/Engine/EditorBlueprintResources/StandardMacros.IsValid` _returnvalue
    (:`Is Valid`
      (`SceneComponent.K2_SetWorldRotation` _ammo_sprite (`KismetMathLibrary.MakeRotator` 0.0 0.0 (- _returnvalue_yaw 90.0)) false false))))

(event `/Game/DirtyManners/Blueprints/Interfaces/BPI_Interactable.On Interact`
  (bind _returnvalue (`GameplayStatics.GetPlayerPawn` 0))
  (bind _returnvalue_2 (`GameplayStatics.GetPlayerPawn` 0))
  (bind _returnvalue_3 (`GameplayStatics.GetPlayerPawn` 0))
  (bind _returnvalue_4 (`|GetDataTableRow` "/Game/DirtyManners/Blueprints/Weapons/DT_DirtyMannersWeapons.DT_DirtyMannersWeapons" (`KismetStringLibrary.Conv_StringToName` (`KismetStringLibrary.Conv_IntToString` (`self.Weapon Index`))))
    (:`then`
      (switch `/Game/DirtyManners/Blueprints/Enums/ENUM_WeaponList` (`.WeaponName_2_ED9A753648A3CF613FAE83B21A06C6AA` (break `/Game/DirtyManners/Blueprints/Structs/ST_WeaponData` _returnvalue_4))
        (:`NewEnumerator0`
          (bind _asbp_dirty_manners_character (cast `/Game/DirtyManners/Blueprints/BP_DirtyMannersCharacter` _returnvalue_2))
          (if (not (>= (`.ReturnValue` (`AbilitySystemBlueprintLibrary.GetFloatAttributeFromAbilitySystemComponent` (`AbilitySystemBlueprintLibrary.GetAbilitySystemComponent` _returnvalue_2) (struct :`AttributeName` "Bullets" :`Attribute` "/Script/Dirty_Manners.DirtyMannersAttributeSet:Bullets" :`AttributeOwner` "/Script/CoreUObject.Class'/Script/Dirty_Manners.DirtyMannersAttributeSet'"))) (`DirtyMannersCharacter.MaxBullets` _asbp_dirty_manners_character)))
            (bind _asbp_fpsplayer (cast `/Game/DirtyManners/Blueprints/Player/BP_FPSPlayer` (`GameplayStatics.GetPlayerPawn` 0) :!label _label))
            (`/Game/DirtyManners/Blueprints/Player/BP_FPSPlayer.Weapon Pickup` _asbp_fpsplayer (`.WeaponName_2_ED9A753648A3CF613FAE83B21A06C6AA` (break `/Game/DirtyManners/Blueprints/Structs/ST_WeaponData` _returnvalue_4)))
            (`GameplayStatics.PlaySoundAtLocation` "/Game/DirtyManners/SFX/Buy_SFX.Buy_SFX" (`SceneComponent.K2_GetComponentLocation` (`self.DefaultSceneRoot`)) (struct) 0.3 1.0 0.0 null null null null)))
        (:`NewEnumerator1`
          (bind _asbp_dirty_manners_character_2 (cast `/Game/DirtyManners/Blueprints/BP_DirtyMannersCharacter` _returnvalue))
          (if (not (>= (`.ReturnValue` (`AbilitySystemBlueprintLibrary.GetFloatAttributeFromAbilitySystemComponent` (`AbilitySystemBlueprintLibrary.GetAbilitySystemComponent` _returnvalue) (struct :`AttributeName` "Rockets" :`Attribute` "/Script/Dirty_Manners.DirtyMannersAttributeSet:Rockets" :`AttributeOwner` "/Script/CoreUObject.Class'/Script/Dirty_Manners.DirtyMannersAttributeSet'"))) (`DirtyMannersCharacter.MaxRockets` _asbp_dirty_manners_character_2)))
            (goto _label)))
        (:`NewEnumerator3`
          (bind _asbp_dirty_manners_character_3 (cast `/Game/DirtyManners/Blueprints/BP_DirtyMannersCharacter` _returnvalue_3))
          (if (not (>= (`.ReturnValue` (`AbilitySystemBlueprintLibrary.GetFloatAttributeFromAbilitySystemComponent` (`AbilitySystemBlueprintLibrary.GetAbilitySystemComponent` _returnvalue_3) (struct :`AttributeName` "Soap" :`Attribute` "/Script/Dirty_Manners.DirtyMannersAttributeSet:Soap" :`AttributeOwner` "/Script/CoreUObject.Class'/Script/Dirty_Manners.DirtyMannersAttributeSet'"))) (`DirtyMannersCharacter.MaxSoap` _asbp_dirty_manners_character_3)))
            (goto _label)))))))

(fn `Is interactable / Details`
  (returns (`Interaction Type` :type "/Game/DirtyManners/Blueprints/Enums/ENUM_InteractableList Enum") (Text :type Text) (Price :type Integer) (WeaponIndex :type Integer))
  (bind _weapon_index (`self.Weapon Index`))
  (bind _returnvalue (`|GetDataTableRow` "/Game/DirtyManners/Blueprints/Weapons/DT_DirtyMannersWeapons.DT_DirtyMannersWeapons" (`KismetStringLibrary.Conv_StringToName` (`KismetStringLibrary.Conv_IntToString` _weapon_index)))
    (:`then`
      (return "NewEnumerator2" (`|GenericToText` (`.AmmoType_11_EEA65B6B42CC75F1669908828DE25C61` (break `/Game/DirtyManners/Blueprints/Structs/ST_WeaponData` _returnvalue))) 500 _weapon_index))))

(fn `UserConstructionScript`)