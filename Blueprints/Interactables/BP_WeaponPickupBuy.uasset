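; Purchasable weapon spawner interactable that, when interacted with, replaces itself with a BP_WeaponPickup for its weapon and plays a buy sound.
; WeaponIndex keys a DT_DirtyMannersWeapons row that sets the display flipbook, the spawned weapon and the interaction prompt.
; The prompt details report a fixed price, and no payment is handled in this Blueprint.
; The flipbook billboards on yaw toward the player camera every tick.
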(event `self.ReceiveBeginPlay`
  (bind _pickup_flipbook (`self.Pickup Flipbook`))
  (bind _returnvalue (`|GetDataTableRow` "/Game/DirtyManners/Blueprints/Weapons/DT_DirtyMannersWeapons.DT_DirtyMannersWeapons" (`KismetStringLibrary.Conv_StringToName` (`KismetStringLibrary.Conv_IntToString` (`self.Weapon Index`))))
    (:`then`
      (switch `/Game/DirtyManners/Blueprints/Enums/ENUM_WeaponList` (`.WeaponName_2_ED9A753648A3CF613FAE83B21A06C6AA` (break `/Game/DirtyManners/Blueprints/Structs/ST_WeaponData` _returnvalue))
        (:`NewEnumerator2`
          (`PaperFlipbookComponent.SetFlipbook` _pickup_flipbook null))
        (:`NewEnumerator0`
          (`PaperFlipbookComponent.SetFlipbook` _pickup_flipbook "/Game/DirtyManners/Flipbooks/FB_InteractablePickup_SprayBottle.FB_InteractablePickup_SprayBottle"))
        (:`NewEnumerator1`
          (`PaperFlipbookComponent.SetFlipbook` _pickup_flipbook "/Game/DirtyManners/Flipbooks/FB_InteractablePickup_Launcher.FB_InteractablePickup_Launcher"))
        (:`NewEnumerator3`
          (`PaperFlipbookComponent.SetFlipbook` _pickup_flipbook "/Game/DirtyManners/Flipbooks/FB_InteractableSpawner_Bubbler.FB_InteractableSpawner_Bubbler"))))))

(event `self.ReceiveTick`
  (params (DeltaSeconds :type "Float (single-precision)"))
  (bind _returnvalue (`GameplayStatics.GetPlayerCameraManager` 0))
  (bind _pickup_flipbook (`self.Pickup Flipbook`))
  (bind (_returnvalue_roll _returnvalue_pitch _returnvalue_yaw) (`KismetMathLibrary.BreakRotator` (`KismetMathLibrary.FindLookAtRotation` (`SceneComponent.K2_GetComponentLocation` _pickup_flipbook) (`PlayerCameraManager.GetCameraLocation` _returnvalue))))
  (`/Engine/EditorBlueprintResources/StandardMacros.IsValid` _returnvalue
    (:`Is Valid`
      (`SceneComponent.K2_SetWorldRotation` _pickup_flipbook (`KismetMathLibrary.MakeRotator` 0.0 0.0 (- _returnvalue_yaw 90.0)) false false))))

(event `/Game/DirtyManners/Blueprints/Interfaces/BPI_Interactable.On Interact`
  (bind _returnvalue (`|GetDataTableRow` "/Game/DirtyManners/Blueprints/Weapons/DT_DirtyMannersWeapons.DT_DirtyMannersWeapons" (`KismetStringLibrary.Conv_StringToName` (`KismetStringLibrary.Conv_IntToString` (`self.Weapon Index`))))
    (:`then`
      (`|SpawnActorFromClass` "/Game/DirtyManners/Blueprints/Pickups/BP_WeaponPickup.BP_WeaponPickup_C" (`KismetMathLibrary.MakeTransform` (`SceneComponent.K2_GetComponentLocation` (`self.DefaultSceneRoot`))) "Undefined" "MultiplyWithRoot" null (`.WeaponName_2_ED9A753648A3CF613FAE83B21A06C6AA` (break `/Game/DirtyManners/Blueprints/Structs/ST_WeaponData` _returnvalue)) null)
      (`GameplayStatics.PlaySoundAtLocation` "/Game/DirtyManners/SFX/Buy_SFX.Buy_SFX" (`SceneComponent.K2_GetComponentLocation` (`self.DefaultSceneRoot`)) (struct) 0.3 1.0 0.0 null null null null)
      (`self.K2_DestroyActor`))))

(fn `Is interactable / Details`
  (returns (`Interaction Type` :type "/Game/DirtyManners/Blueprints/Enums/ENUM_InteractableList Enum") (Text :type Text) (Price :type Integer) (WeaponIndex :type Integer))
  (bind _weapon_index (`self.Weapon Index`))
  (bind _returnvalue (`|GetDataTableRow` "/Game/DirtyManners/Blueprints/Weapons/DT_DirtyMannersWeapons.DT_DirtyMannersWeapons" (`KismetStringLibrary.Conv_StringToName` (`KismetStringLibrary.Conv_IntToString` _weapon_index)))
    (:`then`
      (return "NewEnumerator2" (`|FormatText` "{Weapon name} Spawner" (`|GenericToText` (`.WeaponName_2_ED9A753648A3CF613FAE83B21A06C6AA` (break `/Game/DirtyManners/Blueprints/Structs/ST_WeaponData` _returnvalue)))) 1000 _weapon_index))))

(fn `UserConstructionScript`)