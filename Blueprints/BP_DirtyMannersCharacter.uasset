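; Base character Blueprint that handles damage and death through the Gameplay Ability System.
; TakeDamage receives cue data and reports a damage event with instigator and location, likely for AI sense perception.
; It then reads an ability system attribute through HealthCheck and calls KillCharacter at zero or below.
; KillCharacter is empty here, and the debug health and armor prints are disconnected.
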(event `Take Damage`
  (params (`Cue Data` :type "GameplayCueParameters Structure"))
  (bind (_normalizedmagnitude _rawmagnitude _effectcontext _matchedtagname _originaltag _aggregatedsourcetags _aggregatedtargettags _location) (`AbilitySystemBlueprintLibrary.BreakGameplayCueParameters` `Cue Data`))
  (`AISense_Damage.ReportDamageEvent` self (`AbilitySystemBlueprintLibrary.EffectContextGetInstigatorActor` _effectcontext) 0.0 _location)
  (if (`self.Health Check`)
    (`self.Kill Character`)))

(event `Kill Character`)

(fn `Health Check`
  (returns (`IsDead?` :type Boolean))
  (return (<= (`.ReturnValue` (`AbilitySystemBlueprintLibrary.GetFloatAttributeFromAbilitySystemComponent` (`self.AbilitySystemComponent`) (struct :`AttributeName` "Health" :`Attribute` "/Script/Dirty_Manners.DirtyMannersAttributeSet:Health" :`AttributeOwner` "/Script/CoreUObject.Class'/Script/Dirty_Manners.DirtyMannersAttributeSet'"))) 0.0)))

(fn `UserConstructionScript`)