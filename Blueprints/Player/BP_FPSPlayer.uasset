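; First-person player character that handles movement, look, weapons, pickups, HUD updates and point-based purchases.
; Weapons come from a data table, spawn as child actors beside a mop melee weapon, and fire or gain ammo through GAS abilities activated by gameplay tags.
; A per-tick camera trace finds interactables and sets buy prompts, charging a quarter price for owned weapons.
; Damage and pickups refresh the HUD with colour flashes, and death shows a death screen.
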(event `self.ReceiveBeginPlay`
  ; Initialization
  (`parent.ReceiveBeginPlay`)
  (bind _returnvalue (`|CreateWidget` "/Game/DirtyManners/Blueprints/Widgets/WBP_Hud.WBP_Hud_C"))
  (bind _output_get (set `self.HUD` _returnvalue))
  (`UserWidget.AddToViewport` _output_get 0)
  (`KismetSystemLibrary.Delay` 0.0)
  (`self.Update UI`)
  (`self.Initialize Weapon` "/Game/DirtyManners/Blueprints/Player/BP_PlayerWeaponBase.BP_PlayerWeaponBase_C")
  (`/Game/DirtyManners/Blueprints/Widgets/WBP_Hud.Switch Weapon` (`self.HUD`) "NewEnumerator2")
  (`self.Initialize Melee Weapon` "/Game/DirtyManners/Blueprints/Weapons/BP_Mop.BP_Mop_C"))

(event `InputAxis|HorizontalMovement`
  (params (AxisValue :type "Float (single-precision)"))
  (bind (_returnvalue_roll _returnvalue_pitch _returnvalue_yaw) (`KismetMathLibrary.BreakRotator` (`self.GetControlRotation`)))
  ; Movement Section
  (`self.AddMovementInput` (`KismetMathLibrary.GetRightVector` (`KismetMathLibrary.MakeRotator` 0.0 0.0 _returnvalue_yaw)) AxisValue))

(event `self.ReceiveTick`
  (params (DeltaSeconds :type "Float (single-precision)"))
  ; Weapon bobbing animation
  (bind _asbp_player_weapon_base (cast `/Game/DirtyManners/Blueprints/Player/BP_PlayerWeaponBase` (`ChildActorComponent.ChildActor` (`self.Weapon`))))
  (`/Game/DirtyManners/Blueprints/Player/BP_PlayerWeaponBase.Weapon bobbing` _asbp_player_weapon_base (> (`KismetMathLibrary.VSize` (`MovementComponent.Velocity` (`self.CharacterMovement`))) 0.0) DeltaSeconds)
  (`self.Interact Set Text`))

(event `InputAxis|VerticalMovement`
  (params (AxisValue :type "Float (single-precision)"))
  (bind (_returnvalue_roll _returnvalue_pitch _returnvalue_yaw) (`KismetMathLibrary.BreakRotator` (`self.GetControlRotation`)))
  ; Movement Section
  (`self.AddMovementInput` (`KismetMathLibrary.GetForwardVector` (`KismetMathLibrary.MakeRotator` 0.0 0.0 _returnvalue_yaw)) AxisValue))

(event `InputAction|Interaction`
  (params (Key :type "Key Structure"))
  (bind _interaction_price (`self.Interaction Price`))
  (bind _hud (`self.HUD`))
  (bind _hud_2 (`self.HUD`))
  (bind _interaction_price_2 (`self.Interaction Price`))
  (bind _interaction_hit_actor (`self.Interaction Hit Actor`))
  ; Interaction system
  (:`Pressed`
    (bind _interact_type (`self.Interact Trace`))
    (switch `/Game/DirtyManners/Blueprints/Enums/ENUM_InteractableList` _interact_type
      (:`NewEnumerator2`
        (if (>= (`/Game/DirtyManners/Blueprints/Widgets/WBP_Hud.CurrentPoints` (`self.HUD`)) (`KismetMathLibrary.SelectInt` (/ _interaction_price_2 4) _interaction_price_2 (`self.Has Weapon ?` "NewEnumerator2" (`self.Interaction Weapon Index`))))
          (`UserWidget.PlayAnimation` _hud_2 (`/Game/DirtyManners/Blueprints/Widgets/WBP_Hud.InteractionAccept` _hud_2) 0.0 1 "Forward" 1.0 false)
          (`/Game/DirtyManners/Blueprints/Widgets/WBP_Hud.Decrease Points` (`self.HUD`) (`KismetMathLibrary.SelectInt` (/ _interaction_price 4) _interaction_price (`self.Has Weapon ?` "NewEnumerator2" (`self.Interaction Weapon Index`))))
          (`/Engine/EditorBlueprintResources/StandardMacros.IsValid` _interaction_hit_actor
            (:`Is Valid`
              (message `/Game/DirtyManners/Blueprints/Interfaces/BPI_Interactable.On Interact` _interaction_hit_actor)))
          (else
            (`UserWidget.PlayAnimation` _hud (`/Game/DirtyManners/Blueprints/Widgets/WBP_Hud.InteractionDecline` _hud) 0.0 1 "Forward" 1.0 false)))))))

(event `InputAction|SwitchPistol`
  (params (Key :type "Key Structure"))
  ; Weapon Switching
  (:`Pressed`
    (if (`self.Has Weapon ?` "NewEnumerator0")
      (bind _weapon_data (`self.Get Weapon From Data Table` "NewEnumerator0"))
      (`self.Equip Weapon` _weapon_data))))

(event `InputAxis|MouseLookHorizontal`
  (params (AxisValue :type "Float (single-precision)"))
  ; Mouse Look Section
  (`self.AddControllerYawInput` AxisValue))

(event `InputAction|SwitchLauncher`
  (params (Key :type "Key Structure"))
  ; Weapon Switching
  (:`Pressed`
    (if (`self.Has Weapon ?` "NewEnumerator1")
      (bind _weapon_data (`self.Get Weapon From Data Table` "NewEnumerator1"))
      (`self.Equip Weapon` _weapon_data))))

(event `InputAxis|MouseLookVertical`
  (params (AxisValue :type "Float (single-precision)"))
  ; Mouse Look Section
  (`self.AddControllerPitchInput` AxisValue))

(event `InputAction|SwitchBubbler`
  (params (Key :type "Key Structure"))
  ; Weapon Switching
  (:`Pressed`
    (if (`self.Has Weapon ?` "NewEnumerator3")
      (bind _weapon_data (`self.Get Weapon From Data Table` "NewEnumerator3"))
      (`self.Equip Weapon` _weapon_data))))

(event `InputAction|FireWeapon`
  (params (Key :type "Key Structure"))
  ; Weapon Fire
  (:`Pressed`
    (`AbilitySystemComponent.TryActivateAbilitiesByTag` (`self.AbilitySystemComponent`) (`self.Weapon Fire Tag Container`) false)))

(event `Equip Weapon`
  (params (Weapon :type "/Game/DirtyManners/Blueprints/Structs/ST_WeaponData Structure"))
  (bind (_currentweapon_weaponindex _currentweapon_weaponname) (break `/Game/DirtyManners/Blueprints/Structs/ST_WeaponData` (`self.CurrentWeapon`)))
  ; Equip Weapon
  (bind _output_get (set `self.CurrentWeapon` Weapon))
  (bind _weapon_actor (`self.Initialize Weapon` (`.Weapon_5_8A52AC2444BB602BF47F84B701177634` (break `/Game/DirtyManners/Blueprints/Structs/ST_WeaponData` _output_get))))
  (bind _asbp_player_weapon_base (cast `/Game/DirtyManners/Blueprints/Player/BP_PlayerWeaponBase` _weapon_actor))
  ; Equip animation
  (`MovieSceneSequencePlayer.Play` (`ActorSequenceComponent.SequencePlayer` (`/Game/DirtyManners/Blueprints/Player/BP_PlayerWeaponBase.Weapon draw` _asbp_player_weapon_base)))
  ; Gameplay Tag Setup
  (`/Game/DirtyManners/Blueprints/Widgets/WBP_Hud.Switch Weapon` (`self.HUD`) _currentweapon_weaponname)
  (`self.Update UI`)
  (switch `/Game/DirtyManners/Blueprints/Enums/ENUM_WeaponList` _currentweapon_weaponname
    (:`NewEnumerator2`
      (set `self.Weapon Fire Tag Container` (struct)))
    (:`NewEnumerator0`
      (set `self.Weapon Fire Tag Container` (struct :`GameplayTags` (struct :`(TagName` "Player.Weapon.Pistol.Fire")))))
    (:`NewEnumerator1`
      (set `self.Weapon Fire Tag Container` (struct :`GameplayTags` (struct :`(TagName` "Player.Weapon.Launcher.Fire")))))
    (:`NewEnumerator3`
      (set `self.Weapon Fire Tag Container` (struct :`GameplayTags` (struct :`(TagName` "Player.Weapon.Bubbler.FIre")))))))

(event `self.Kill Character`
  ; Death Screen
  (`Widget.SetVisibility` (`self.HUD`) "Hidden")
  (bind _returnvalue (`|CreateWidget` "/Game/DirtyManners/Blueprints/Widgets/WBP_DeathScreen.WBP_DeathScreen_C"))
  (`UserWidget.AddToViewport` _returnvalue 0))

(event `self.Take Damage`
  (params (`Cue Data` :type "GameplayCueParameters Structure"))
  ; Damage Taken
  (`parent.Take Damage` `Cue Data`)
  (`self.Update UI`)
  (bind (_direction _alpha) (`Timeline|Damage Flash` :!via `PlayFromStart`)
    (:`Update`
      (`/Game/DirtyManners/Blueprints/Widgets/WBP_Hud.Set Flash Color` (`self.HUD`) (struct :`R` 1.0 :`B` 0.003628 :`A` 1.0) _alpha))))

(event `Item Pickup`
  ; Item Pickup
  (`self.Update UI`)
  (bind (_direction _alpha) (`Timeline|Pickup Flash` :!via `PlayFromStart`)
    (:`Update`
      (`/Game/DirtyManners/Blueprints/Widgets/WBP_Hud.Set Flash Color` (`self.HUD`) (struct :`R` 0.057993 :`G` 1.0 :`B` 0.179412 :`A` 1.0) _alpha))))

(event `Weapon Pickup`
  (params (Weapon :type "/Game/DirtyManners/Blueprints/Enums/ENUM_WeaponList Enum" :default "NewEnumerator2"))
  ; Weapon Pickup
  (bind (_weapon_data _weapon_found) (`self.Get Weapon From Data Table` Weapon))
  (if _weapon_found
    (bind _output_get (set `self.Weapon To Pickup` _weapon_data))
    (bind (_weaponindex _weaponname _weapon _ammotype _ammosize) (break `/Game/DirtyManners/Blueprints/Structs/ST_WeaponData` _output_get))
    (if (`self.Has Weapon ?` _weaponname)
      (`self.Add Ammo` _ammotype _ammosize)
      (else
        (`self.Add Weapon`)))
    (else
      (`KismetSystemLibrary.PrintString` "Weapon Does Not Exist In Data Table"))))

(event `Add Ammo`
  (params (`Ammo Type` :type "/Game/DirtyManners/Blueprints/Enums/ENUM_AmmoList Enum" :default "NewEnumerator2") (`Pikcup Size` :type "/Game/DirtyManners/Blueprints/Enums/ENUM_PickupSize Enum" :default "NewEnumerator0"))
  ; Add Ammo
  (switch `/Game/DirtyManners/Blueprints/Enums/ENUM_AmmoList` `Ammo Type`
    (:`NewEnumerator0`
      (`self.Add Bullets` `Pikcup Size`))
    (:`NewEnumerator1`
      (`self.Add Rockets` `Pikcup Size`))
    (:`NewEnumerator3`
      (`self.Add Soap` `Pikcup Size`))))

(event `Add Weapon`
  (bind _weapon_to_pickup (`self.Weapon To Pickup`))
  (bind (_weaponindex _weaponname _weapon _ammotype _ammosize) (break `/Game/DirtyManners/Blueprints/Structs/ST_WeaponData` _weapon_to_pickup))
  ; Add Weapon
  (`KismetArrayLibrary.Array_Add` (`self.Player Weapons`) _weapon_to_pickup)
  (`self.Equip Weapon` _weapon_to_pickup)
  (`self.Add Ammo` _ammotype _ammosize))

(event `InputAction|MeleeAttack`
  (params (Key :type "Key Structure"))
  ; Meee Attack
  (:`Pressed`
    (`AbilitySystemComponent.TryActivateAbilitiesByTag` (`self.AbilitySystemComponent`) (`self.Melee Fire Tag Container`) false)))

(fn `Add Bullets`
  (params (`Pickup Size` :type "/Game/DirtyManners/Blueprints/Enums/ENUM_PickupSize Enum" :default "NewEnumerator0"))
  (if (not (>= (`.ReturnValue` (`AbilitySystemBlueprintLibrary.GetFloatAttributeFromAbilitySystemComponent` (`self.AbilitySystemComponent`) (struct :`AttributeName` "Bullets" :`Attribute` "/Script/Dirty_Manners.DirtyMannersAttributeSet:Bullets" :`AttributeOwner` "/Script/CoreUObject.Class'/Script/Dirty_Manners.DirtyMannersAttributeSet'"))) (`self.MaxBullets`)))
    (switch `/Game/DirtyManners/Blueprints/Enums/ENUM_PickupSize` `Pickup Size`
      (:`NewEnumerator0`
        (set `self.Ammo Gain Tag Container` (struct :`GameplayTags` (struct :`(TagName` "Pickup.Ammo.Bullets.Small"))))
        (`AbilitySystemComponent.TryActivateAbilitiesByTag` (`self.AbilitySystemComponent`) (`self.Ammo Gain Tag Container`) true)
        (`self.Item Pickup`)))))

(fn `Add Rockets`
  (params (`Pickup Size` :type "/Game/DirtyManners/Blueprints/Enums/ENUM_PickupSize Enum" :default "NewEnumerator0"))
  (if (not (>= (`.ReturnValue` (`AbilitySystemBlueprintLibrary.GetFloatAttributeFromAbilitySystemComponent` (`self.AbilitySystemComponent`) (struct :`AttributeName` "Rockets" :`Attribute` "/Script/Dirty_Manners.DirtyMannersAttributeSet:Rockets" :`AttributeOwner` "/Script/CoreUObject.Class'/Script/Dirty_Manners.DirtyMannersAttributeSet'"))) (`self.MaxRockets`)))
    (switch `/Game/DirtyManners/Blueprints/Enums/ENUM_PickupSize` `Pickup Size`
      (:`NewEnumerator0`
        (set `self.Ammo Gain Tag Container` (struct :`GameplayTags` (struct :`(TagName` "Pickup.Ammo.Rockets.Small"))))
        (`AbilitySystemComponent.TryActivateAbilitiesByTag` (`self.AbilitySystemComponent`) (`self.Ammo Gain Tag Container`) true)
        (`self.Item Pickup`)))))

(fn `Add Soap`
  (params (`Pickup Size` :type "/Game/DirtyManners/Blueprints/Enums/ENUM_PickupSize Enum" :default "NewEnumerator0"))
  (if (not (>= (`.ReturnValue` (`AbilitySystemBlueprintLibrary.GetFloatAttributeFromAbilitySystemComponent` (`self.AbilitySystemComponent`) (struct :`AttributeName` "Soap" :`Attribute` "/Script/Dirty_Manners.DirtyMannersAttributeSet:Soap" :`AttributeOwner` "/Script/CoreUObject.Class'/Script/Dirty_Manners.DirtyMannersAttributeSet'"))) (`self.MaxSoap`)))
    (switch `/Game/DirtyManners/Blueprints/Enums/ENUM_PickupSize` `Pickup Size`
      (:`NewEnumerator0`
        (set `self.Ammo Gain Tag Container` (struct :`GameplayTags` (struct :`(TagName` "Pickup.Ammo.Soap.Small"))))
        (`AbilitySystemComponent.TryActivateAbilitiesByTag` (`self.AbilitySystemComponent`) (`self.Ammo Gain Tag Container`) true)
        (`self.Item Pickup`)))))

(fn `Get Weapon From Data Table`
  (params (Weapon :type "/Game/DirtyManners/Blueprints/Enums/ENUM_WeaponList Enum" :default "NewEnumerator2"))
  (returns (`Weapon Data` :type "/Game/DirtyManners/Blueprints/Structs/ST_WeaponData Structure") (`Weapon Found` :type Boolean))
  (locals (`Weapon Exists` :type Boolean) (`Weapon To Equip` :type "/Game/DirtyManners/Blueprints/Structs/ST_WeaponData Structure"))
  (bind _outrownames (`DataTableFunctionLibrary.GetDataTableRowNames` "/Game/DirtyManners/Blueprints/Weapons/DT_DirtyMannersWeapons.DT_DirtyMannersWeapons"))
  (for _array_element _outrownames
    (bind _returnvalue (`|GetDataTableRow` "/Game/DirtyManners/Blueprints/Weapons/DT_DirtyMannersWeapons.DT_DirtyMannersWeapons" _array_element)
      (:`then`
        (if (`|EnumEquality` Weapon (`.WeaponName_2_ED9A753648A3CF613FAE83B21A06C6AA` (break `/Game/DirtyManners/Blueprints/Structs/ST_WeaponData` _returnvalue)))
          (set `local.Weapon Exists` true)
          (set `local.Weapon To Equip` _returnvalue)
          (break)))))
  (return (`local.Weapon To Equip`) (`local.Weapon Exists`)))

(fn `Has Weapon ?`
  (params (`Weapon Type` :type "/Game/DirtyManners/Blueprints/Enums/ENUM_WeaponList Enum" :default "NewEnumerator2") (Index :type Integer))
  (returns (`Has Weapon ?` :type Boolean) (`Weapon Index` :type Integer))
  (locals (`Has Weapon` :type Boolean))
  (for _array_element (`self.Player Weapons`)
    (bind (_weaponindex _weaponname) (break `/Game/DirtyManners/Blueprints/Structs/ST_WeaponData` _array_element))
    (if (or (`|EnumEquality` _weaponname `Weapon Type`) (== _weaponindex Index))
      (set `local.Has Weapon` true)
      (break)))
  (return (`local.Has Weapon`) _weaponindex))

(fn `Initialize Melee Weapon`
  (params (`In Class` :type "/Game/DirtyManners/Blueprints/Player/BP_PlayerMeleeWeaponBase Class Reference"))
  (returns (`Weapon Actor` :type "Actor Object Reference"))
  (bind _melee_weapon (`self.Melee Weapon`))
  (bind _childactor (`ChildActorComponent.ChildActor` _melee_weapon))
  (`ChildActorComponent.SetChildActorClass` _melee_weapon `In Class`)
  (if (`KismetSystemLibrary.DoesImplementInterface` _childactor "/Game/DirtyManners/Blueprints/Interfaces/BPI_PlayerWeapon.BPI_PlayerWeapon_C")
    (message `/Game/DirtyManners/Blueprints/Interfaces/BPI_PlayerWeapon.InitializeWeapon` _childactor))
  (return _childactor))

(fn `Initialize Weapon`
  (params (`In Class` :type "/Game/DirtyManners/Blueprints/Player/BP_PlayerWeaponBase Class Reference"))
  (returns (`Weapon Actor` :type "Actor Object Reference"))
  (bind _weapon (`self.Weapon`))
  (bind _childactor (`ChildActorComponent.ChildActor` _weapon))
  (`ChildActorComponent.SetChildActorClass` _weapon `In Class`)
  (if (`KismetSystemLibrary.DoesImplementInterface` _childactor "/Game/DirtyManners/Blueprints/Interfaces/BPI_PlayerWeapon.BPI_PlayerWeapon_C")
    (message `/Game/DirtyManners/Blueprints/Interfaces/BPI_PlayerWeapon.InitializeWeapon` _childactor))
  (return _childactor))

(fn `Interact Set Text`
  (bind _interaction_weapon_index (`self.Interaction Weapon Index`))
  (bind _interact_type (`self.Interact Trace`))
  (switch `/Game/DirtyManners/Blueprints/Enums/ENUM_InteractableList` _interact_type
    (:`NewEnumerator1`
      (set `TextBlock.Text` (`|FormatText` "Press E to {Interaction Text}" (`self.Interaction Text`)) (`/Game/DirtyManners/Blueprints/Widgets/WBP_Hud.InteractionText` (`self.HUD`))))
    (:`NewEnumerator2`
      (if (> _interaction_weapon_index 0)
        (`|GetDataTableRow` "/Game/DirtyManners/Blueprints/Weapons/DT_DirtyMannersWeapons.DT_DirtyMannersWeapons" (`KismetStringLibrary.Conv_StringToName` (`KismetStringLibrary.Conv_IntToString` _interaction_weapon_index))
          (:`then`
            (set `TextBlock.Text` (select `bool` (`self.Has Weapon ?` "NewEnumerator2" (`self.Interaction Weapon Index`)) :`false` (`|FormatText` "Press E to Buy {Weapon Name} for {amount} points" (`self.Interaction Text`) (`self.Interaction Price`)) :`true` (`|FormatText` "Press E to Buy {Ammo Name} for {amount} points" (`self.Interaction Text`) (/ (`self.Interaction Price`) 4))) (`/Game/DirtyManners/Blueprints/Widgets/WBP_Hud.InteractionText` (`self.HUD`)))))
        (else
          (`KismetSystemLibrary.PrintString` "Missing Weapon Index"))))))

(fn `Interact Trace`
  (returns (`Interact Type` :type "/Game/DirtyManners/Blueprints/Enums/ENUM_InteractableList Enum"))
  (bind _camera (`self.Camera`))
  (bind _returnvalue (`SceneComponent.K2_GetComponentLocation` _camera))
  (bind _outhit (`KismetSystemLibrary.LineTraceSingle` _returnvalue (+ _returnvalue (* (`SceneComponent.GetForwardVector` _camera) 250.0)) "TraceTypeQuery1"))
  (if (`KismetSystemLibrary.DoesImplementInterface` (`.HitActor` (`GameplayStatics.BreakHitResult` _outhit)) "/Game/DirtyManners/Blueprints/Interfaces/BPI_Interactable.BPI_Interactable_C")
    (set `self.Interaction Hit Actor` (`.HitActor` (`GameplayStatics.BreakHitResult` _outhit)))
    (bind (_interaction_type _text _price _weaponindex) (message `/Game/DirtyManners/Blueprints/Interfaces/BPI_Interactable.Is interactable / Details` (`self.Interaction Hit Actor`)))
    (`|ExecutionSequence`
      (:`then_0`
        (set `self.Interaction Text` _text)
        (set `self.Interaction Price` _price)
        (set `self.Interaction Weapon Index` _weaponindex))
      (:`then_1`
        (set `self.Interacting` true)
        (return _interaction_type)))
    (elif (`self.Interacting`)
      (set `TextBlock.Text` "" (`/Game/DirtyManners/Blueprints/Widgets/WBP_Hud.InteractionText` (`self.HUD`)))
      (set `self.Interacting` false))))

(fn `Update UI`
  (bind _abilitysystemcomponent (`self.AbilitySystemComponent`))
  (bind _hud (`self.HUD`))
  (bind _currentammo (`/Game/DirtyManners/Blueprints/Widgets/WBP_Hud.CurrentAmmo` (`self.HUD`)))
  (`TextBlock.SetText` (`/Game/DirtyManners/Blueprints/Widgets/WBP_Hud.HealthValue` _hud) (`KismetTextLibrary.Conv_DoubleToText` (`.ReturnValue` (`AbilitySystemBlueprintLibrary.GetFloatAttributeFromAbilitySystemComponent` _abilitysystemcomponent (struct :`AttributeName` "Health" :`Attribute` "/Script/Dirty_Manners.DirtyMannersAttributeSet:Health" :`AttributeOwner` "/Script/CoreUObject.Class'/Script/Dirty_Manners.DirtyMannersAttributeSet'"))) "HalfToEven"))
  (`TextBlock.SetText` (`/Game/DirtyManners/Blueprints/Widgets/WBP_Hud.ArmorValue` _hud) (`KismetTextLibrary.Conv_DoubleToText` (`.ReturnValue` (`AbilitySystemBlueprintLibrary.GetFloatAttributeFromAbilitySystemComponent` _abilitysystemcomponent (struct :`AttributeName` "Armor" :`Attribute` "/Script/Dirty_Manners.DirtyMannersAttributeSet:Armor" :`AttributeOwner` "/Script/CoreUObject.Class'/Script/Dirty_Manners.DirtyMannersAttributeSet'"))) "HalfToEven"))
  (switch `/Game/DirtyManners/Blueprints/Enums/ENUM_AmmoList` (`.AmmoType_11_EEA65B6B42CC75F1669908828DE25C61` (break `/Game/DirtyManners/Blueprints/Structs/ST_WeaponData` (`self.CurrentWeapon`)))
    (:`NewEnumerator0`
      (`TextBlock.SetText` _currentammo (`KismetTextLibrary.Conv_DoubleToText` (`.ReturnValue` (`AbilitySystemBlueprintLibrary.GetFloatAttributeFromAbilitySystemComponent` (`self.AbilitySystemComponent`) (struct :`AttributeName` "Bullets" :`Attribute` "/Script/Dirty_Manners.DirtyMannersAttributeSet:Bullets" :`AttributeOwner` "/Script/CoreUObject.Class'/Script/Dirty_Manners.DirtyMannersAttributeSet'"))) "HalfToEven")))
    (:`NewEnumerator1`
      (`TextBlock.SetText` _currentammo (`KismetTextLibrary.Conv_DoubleToText` (`.ReturnValue` (`AbilitySystemBlueprintLibrary.GetFloatAttributeFromAbilitySystemComponent` (`self.AbilitySystemComponent`) (struct :`AttributeName` "Rockets" :`Attribute` "/Script/Dirty_Manners.DirtyMannersAttributeSet:Rockets" :`AttributeOwner` "/Script/CoreUObject.Class'/Script/Dirty_Manners.DirtyMannersAttributeSet'"))) "HalfToEven")))
    (:`NewEnumerator3`
      (`TextBlock.SetText` _currentammo (`KismetTextLibrary.Conv_DoubleToText` (`.ReturnValue` (`AbilitySystemBlueprintLibrary.GetFloatAttributeFromAbilitySystemComponent` (`self.AbilitySystemComponent`) (struct :`AttributeName` "Soap" :`Attribute` "/Script/Dirty_Manners.DirtyMannersAttributeSet:Soap" :`AttributeOwner` "/Script/CoreUObject.Class'/Script/Dirty_Manners.DirtyMannersAttributeSet'"))) "HalfToEven")))))

(fn `UserConstructionScript`)