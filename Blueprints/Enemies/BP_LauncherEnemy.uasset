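; BP_LauncherEnemy is an enemy Blueprint that adds a ranged attack ability and a brief light flash to its parent's behavior.
; RangedAttack runs the parent version, then asks the Ability System Component to activate abilities matching a gameplay tag container.
; It then shows a PointLight and hides it after a short delay, producing a flash with each attack.
; The construction script only calls the parent.
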(event `self.Ranged Attack`
  (`parent.Ranged Attack`)
  (`AbilitySystemComponent.TryActivateAbilitiesByTag` (`self.AbilitySystemComponent`) (`self.Gameplay Tag Container`) true)
  (`SceneComponent.SetHiddenInGame` (`self.PointLight`) false false)
  (`KismetSystemLibrary.Delay` 0.2)
  (`SceneComponent.SetHiddenInGame` (`self.PointLight`) true false))

(fn `UserConstructionScript`
  (`parent.UserConstructionScript`))