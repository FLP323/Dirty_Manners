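; Billboarded Paper2D enemy with Doom-style eight-direction sprites, driven by a behavior tree on BP_DirtyMannersEnemyAI.
; Each tick it yaws the flipbook toward the camera, then picks an idle or walk flipbook from velocity and player angle relative to its facing.
; Damage and ranged-attack animations pause directional updates until they finish.
; Death stops AI and collision, plays dying and dead flipbooks, then destroys the actor; melee is empty.
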(event `self.ReceiveBeginPlay`
  (bind _asbp_dirty_manners_enemy_ai (cast `/Game/DirtyManners/Blueprints/Enemies/AI/BP_DirtyMannersEnemyAI` (`self.GetController`)))
  (`AIController.RunBehaviorTree` _asbp_dirty_manners_enemy_ai (`self.Behavior Tree`)))

(event `self.ReceiveTick`
  (params (DeltaSeconds :type "Float (single-precision)"))
  (`self.Sprite Facing Player`
    (:`Out`
      (if (not (or (`self.IsDead`) (`self.Pause Angle Calculations`)))
        (`self.Get Enemy Angle`
          (:`Out`
            (`self.Chek If Walking`
              (:`Out`
                (`self.Calculate Flipbook`)))))))))

(event `self.Take Damage`
  (params (`Cue Data` :type "GameplayCueParameters Structure"))
  (bind _enemy (`self.Enemy`))
  (`parent.Take Damage` `Cue Data`)
  (if (not (`self.IsDead`))
    (set `self.Pause Angle Calculations` true)
    (`PaperFlipbookComponent.SetFlipbook` _enemy (`self.Damaged`))
    (`KismetSystemLibrary.Delay` (`PaperFlipbookComponent.GetFlipbookLength` _enemy))
    (set `self.Pause Angle Calculations` false)))

(event `self.Kill Character`
  (bind _enemy (`self.Enemy`))
  (`parent.Kill Character`)
  (bind _asbp_dirty_manners_enemy_ai (cast `/Game/DirtyManners/Blueprints/Enemies/AI/BP_DirtyMannersEnemyAI` (`self.GetController`)))
  (`BrainComponent.StopLogic` (`AIController.BrainComponent` _asbp_dirty_manners_enemy_ai) "")
  (set `self.IsDead` true)
  (`PrimitiveComponent.SetCollisionEnabled` (`self.CapsuleComponent`) "NoCollision")
  (`PaperFlipbookComponent.SetFlipbook` _enemy (`self.Dying`))
  (`KismetSystemLibrary.Delay` (`PaperFlipbookComponent.GetFlipbookLength` _enemy))
  (`PaperFlipbookComponent.SetFlipbook` (`self.Enemy`) (`self.Dead`))
  (`KismetSystemLibrary.Delay` 10.0)
  (`self.K2_DestroyActor`))

(event `Melee Attack`)

(event `Ranged Attack`
  (bind _enemy (`self.Enemy`))
  (set `self.Pause Angle Calculations` true)
  (`PaperFlipbookComponent.SetFlipbook` _enemy (`self.Shooting`))
  (`KismetSystemLibrary.Delay` (`PaperFlipbookComponent.GetFlipbookLength` _enemy))
  (set `self.Pause Angle Calculations` false))

(fn `Set Flipbook`
  (params (Walking :type "PaperFlipbook Object Reference") (Idle :type "PaperFlipbook Object Reference"))
  (bind _enemy (`self.Enemy`))
  (if (`self.Is Walking`)
    (`PaperFlipbookComponent.SetFlipbook` _enemy Walking)
    (else
      (`PaperFlipbookComponent.SetFlipbook` _enemy Idle))))

(fn `UserConstructionScript`)