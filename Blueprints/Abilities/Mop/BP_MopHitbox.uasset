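; BP_MopHitbox is a short-lived damage volume for the player's mop attack.
; On overlapping a BP_Enemy it plays a hit sound at the world origin and applies GE_PlayerMopDamage, with the enemy's own Ability System Component as both source and target.
; It then awards points through the FPS player's HUD and destroys itself.
; A Delay on Tick destroys it after about a second otherwise.
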(event `self.ReceiveTick`
  (params (DeltaSeconds :type "Float (single-precision)"))
  (`KismetSystemLibrary.Delay` 1.0)
  (`self.K2_DestroyActor`))

(event `self.Hitbox.OnComponentBeginOverlap`
  (params (OverlappedComponent :type "PrimitiveComponent Object Reference") (OtherActor :type "Actor Object Reference") (OtherComp :type "PrimitiveComponent Object Reference") (OtherBodyIndex :type Integer) (bFromSweep :type Boolean) (SweepResult :type "HitResult Structure (by ref)"))
  (bind _asbp_enemy (cast `/Game/DirtyManners/Blueprints/Enemies/BP_Enemy` OtherActor))
  (`GameplayStatics.PlaySoundAtLocation` "/Game/DirtyManners/SFX/MopHit_SFX.MopHit_SFX" (0.0 0.0 0.0) (struct) 0.3 1.0 0.0 null null null null)
  (bind _returnvalue (`AbilitySystemBlueprintLibrary.GetAbilitySystemComponent` _asbp_enemy))
  (`AbilitySystemComponent.BP_ApplyGameplayEffectToTarget` _returnvalue "/Game/DirtyManners/Blueprints/Abilities/Mop/GE_PlayerMopDamage.GE_PlayerMopDamage_C" _returnvalue 0.0 (`AbilitySystemComponent.MakeEffectContext` _returnvalue))
  (bind _asbp_fpsplayer (cast `/Game/DirtyManners/Blueprints/Player/BP_FPSPlayer` (`GameplayStatics.GetPlayerPawn` 0)))
  (`/Game/DirtyManners/Blueprints/Widgets/WBP_Hud.Increase Points` (`/Game/DirtyManners/Blueprints/Player/BP_FPSPlayer.HUD` _asbp_fpsplayer) 50)
  (`self.K2_DestroyActor`))

(fn `UserConstructionScript`)