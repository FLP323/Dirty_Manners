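; BP_BubbleExplosion is the short-lived explosion effect for the Bubbler ability.
; On BeginPlay it plays a quiet pop sound at the splash collision's relative location, not its world location, then destroys itself after the flipbook's length.
; The splash overlap event is empty; disconnected nodes would apply a Gameplay Effect to an overlapped BP_Enemy through its Ability System Component, so the graph deals no damage.
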(event `self.ReceiveBeginPlay`
  (`GameplayStatics.PlaySoundAtLocation` "/Game/DirtyManners/SFX/Bubble_pop_SFX.Bubble_pop_SFX" (`SceneComponent.RelativeLocation` (`self.Explosion Splash Collision`)) (struct) 0.1 1.0 0.0 null null null null)
  (`KismetSystemLibrary.Delay` (`PaperFlipbookComponent.GetFlipbookLength` (`self.Explosion Flipbook`)))
  (`self.K2_DestroyActor`))

(event `self.Explosion Splash Collision.OnComponentBeginOverlap`
  (params (OverlappedComponent :type "PrimitiveComponent Object Reference") (OtherActor :type "Actor Object Reference") (OtherComp :type "PrimitiveComponent Object Reference") (OtherBodyIndex :type Integer) (bFromSweep :type Boolean) (SweepResult :type "HitResult Structure (by ref)"))
  ; Bubble Explosion damage
)

(fn `UserConstructionScript`)