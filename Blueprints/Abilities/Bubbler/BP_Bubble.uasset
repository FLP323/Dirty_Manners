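; BP_Bubble is the Bubbler ability's projectile, a bubble sprite that damages enemies and bursts on impact.
; Each tick it turns the sprite on yaw only to face the player camera.
; When the projectile stops, an enemy hit applies GE_PlayerBubblerDamage through the enemy's own Ability System Component and adds points to the player's HUD.
; It then spawns BP_BubbleExplosion aligned to the impact normal and destroys itself, as it does for non-enemy hits.
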(event `self.ReceiveTick`
  (params (DeltaSeconds :type "Float (single-precision)"))
  (bind _bubble_sprite (`self.Bubble Sprite`))
  (bind (_returnvalue_roll _returnvalue_pitch _returnvalue_yaw) (`KismetMathLibrary.BreakRotator` (`KismetMathLibrary.FindLookAtRotation` (`SceneComponent.K2_GetComponentLocation` _bubble_sprite) (`PlayerCameraManager.GetCameraLocation` (`GameplayStatics.GetPlayerCameraManager` 0)))))
  (`SceneComponent.K2_SetWorldRotation` _bubble_sprite (`KismetMathLibrary.MakeRotator` 0.0 0.0 (- _returnvalue_yaw 90.0)) false false))

(event `self.ProjectileMovement.OnProjectileStop`
  (params (ImpactResult :type "HitResult Structure (by ref)"))
  (bind _asbp_enemy (cast `/Game/DirtyManners/Blueprints/Enemies/BP_Enemy` ImpactResult_HitActor)
    (:`then`
      (bind _returnvalue (`AbilitySystemBlueprintLibrary.GetAbilitySystemComponent` _asbp_enemy))
      (`AbilitySystemComponent.BP_ApplyGameplayEffectToTarget` _returnvalue "/Game/DirtyManners/Blueprints/Abilities/Bubbler/GE_PlayerBubblerDamage.GE_PlayerBubblerDamage_C" _returnvalue 0.0 (`AbilitySystemComponent.MakeEffectContext` _returnvalue))
      (bind _asbp_fpsplayer (cast `/Game/DirtyManners/Blueprints/Player/BP_FPSPlayer` (`GameplayStatics.GetPlayerPawn` 0)))
      (`/Game/DirtyManners/Blueprints/Widgets/WBP_Hud.Increase Points` (`/Game/DirtyManners/Blueprints/Player/BP_FPSPlayer.HUD` _asbp_fpsplayer) 10))
    (:`CastFailed`
      _))
  (`|SpawnActorFromClass` "/Game/DirtyManners/Blueprints/Abilities/Bubbler/BP_BubbleExplosion.BP_BubbleExplosion_C" (`KismetMathLibrary.MakeTransform` ImpactResult_ImpactPoint (`KismetMathLibrary.Conv_VectorToRotator` ImpactResult_ImpactNormal)) "Undefined" "MultiplyWithRoot" null null)
  (`self.K2_DestroyActor`))

(fn `UserConstructionScript`)