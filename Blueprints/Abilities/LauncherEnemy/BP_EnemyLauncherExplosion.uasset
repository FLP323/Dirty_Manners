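; Explosion actor for the launcher enemy that deals splash damage to the player.
; Overlapping the splash collision applies the GE_EnemyLauncherExplosionDamage gameplay effect through the player's own ability system component, as both source and target.
; The actor destroys itself after a delay equal to the explosion flipbook's length.
; An explosion sound node exists but is disconnected, so it never plays.
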(event `self.ReceiveBeginPlay`
  (`KismetSystemLibrary.Delay` (`PaperFlipbookComponent.GetFlipbookLength` (`self.Explosion Flipbook`)))
  (`self.K2_DestroyActor`))

(event `self.Explosion Splash Collision.OnComponentBeginOverlap`
  (params (OverlappedComponent :type "PrimitiveComponent Object Reference") (OtherActor :type "Actor Object Reference") (OtherComp :type "PrimitiveComponent Object Reference") (OtherBodyIndex :type Integer) (bFromSweep :type Boolean) (SweepResult :type "HitResult Structure (by ref)"))
  (bind _asbp_fpsplayer (cast `/Game/DirtyManners/Blueprints/Player/BP_FPSPlayer` OtherActor))
  (bind _returnvalue (`AbilitySystemBlueprintLibrary.GetAbilitySystemComponent` _asbp_fpsplayer))
  (`AbilitySystemComponent.BP_ApplyGameplayEffectToTarget` _returnvalue "/Game/DirtyManners/Blueprints/Abilities/LauncherEnemy/GE_EnemyLauncherExplosionDamage.GE_EnemyLauncherExplosionDamage_C" _returnvalue 0.0 (`AbilitySystemComponent.MakeEffectContext` _returnvalue)))

(fn `UserConstructionScript`)