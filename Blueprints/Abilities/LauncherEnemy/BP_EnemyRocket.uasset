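; BP_EnemyRocket is the launcher enemy's projectile, drawn as a sprite that yaws each tick to face the player camera like a billboard.
; When projectile movement stops, a hit BP_FPSPlayer receives the GE_EnemyLauncherDamage gameplay effect through its own Ability System Component, acting as both source and target.
; The rocket then spawns BP_EnemyLauncherExplosion at the impact point, oriented to the surface normal, and destroys itself.
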(event `self.ReceiveTick`
  (params (DeltaSeconds :type "Float (single-precision)"))
  (bind _returnvalue (`GameplayStatics.GetPlayerCameraManager` 0))
  (bind _rocket_sprite (`self.Rocket Sprite`))
  (bind (_returnvalue_roll _returnvalue_pitch _returnvalue_yaw) (`KismetMathLibrary.BreakRotator` (`KismetMathLibrary.FindLookAtRotation` (`SceneComponent.K2_GetComponentLocation` _rocket_sprite) (`PlayerCameraManager.GetCameraLocation` _returnvalue))))
  (`/Engine/EditorBlueprintResources/StandardMacros.IsValid` _returnvalue
    (:`Is Valid`
      (`SceneComponent.K2_SetWorldRotation` _rocket_sprite (`KismetMathLibrary.MakeRotator` 0.0 0.0 (- _returnvalue_yaw 90.0)) false false))))

(event `self.ProjectileMovement.OnProjectileStop`
  (params (ImpactResult :type "HitResult Structure (by ref)"))
  (bind _asbp_fpsplayer (cast `/Game/DirtyManners/Blueprints/Player/BP_FPSPlayer` ImpactResult_HitActor)
    (:`then`
      (bind _returnvalue (`AbilitySystemBlueprintLibrary.GetAbilitySystemComponent` _asbp_fpsplayer))
      (`AbilitySystemComponent.BP_ApplyGameplayEffectToTarget` _returnvalue "/Game/DirtyManners/Blueprints/Abilities/LauncherEnemy/GE_EnemyLauncherDamage.GE_EnemyLauncherDamage_C" _returnvalue 0.0 (`AbilitySystemComponent.MakeEffectContext` _returnvalue)))
    (:`CastFailed`
      _))
  (`|SpawnActorFromClass` "/Game/DirtyManners/Blueprints/Abilities/LauncherEnemy/BP_EnemyLauncherExplosion.BP_EnemyLauncherExplosion_C" (`KismetMathLibrary.MakeTransform` ImpactResult_ImpactPoint (`KismetMathLibrary.Conv_VectorToRotator` ImpactResult_ImpactNormal)) "Undefined" "MultiplyWithRoot" null null)
  (`self.K2_DestroyActor`))

(fn `UserConstructionScript`)