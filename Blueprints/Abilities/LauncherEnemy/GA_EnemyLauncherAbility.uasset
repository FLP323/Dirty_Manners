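; Gameplay ability that fires a rocket for the launcher enemy.
; The FireWeapon event spawns BP_EnemyRocket at the transform of the enemy's ProjectileSpawnPoint.
; GetEnemy casts the ability's owner actor to BP_LauncherEnemy and caches it for later calls.
; The activate and end events are disabled placeholders, and nothing in this Blueprint calls FireWeapon.
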(event `self.Fire Weapon`
  (bind _launcher_enemy (`self.Get Enemy`))
  (`|SpawnActorFromClass` "/Game/DirtyManners/Blueprints/Abilities/LauncherEnemy/BP_EnemyRocket.BP_EnemyRocket_C" (`SceneComponent.K2_GetComponentToWorld` (`/Game/DirtyManners/Blueprints/Enemies/BP_Enemy.Projectile Spawn Point` _launcher_enemy)) "Undefined" "MultiplyWithRoot" null null))

(fn `Get Enemy`
  (returns (`Launcher Enemy` :type "/Game/DirtyManners/Blueprints/Enemies/BP_LauncherEnemy Object Reference"))
  (bind _returnvalue_owneractor (break `GameplayAbilityActorInfo` (`self.GetActorInfo`)))
  (`/Engine/EditorBlueprintResources/StandardMacros.IsValid` (`self.Launcher Enemy`)
    (:`Is Valid`
      _)
    (:`Is Not Valid`
      (bind _asbp_launcher_enemy (cast `/Game/DirtyManners/Blueprints/Enemies/BP_LauncherEnemy` _returnvalue_owneractor))
      (bind _output_get (set `self.Launcher Enemy` _asbp_launcher_enemy))))
  (return _output_get))