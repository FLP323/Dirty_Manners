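; BP_RocketExplosion is the short-lived explosion actor for the launcher ability, dealing splash damage to enemies.
; On BeginPlay it plays the explosion sound at the splash collision's relative location, then destroys itself when the flipbook's length has elapsed.
; Enemies overlapping the splash collision receive a GAS damage effect through their own ability system component.
; Each such overlap also adds points to the player's HUD.
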(event `self.ReceiveBeginPlay`
  (`GameplayStatics.PlaySoundAtLocation` "/Game/DirtyManners/SFX/Launcher_Explosion_SFX.Launcher_Explosion_SFX" (`SceneComponent.RelativeLocation` (`self.Explosion Splash Collision`)) (struct) 0.3 1.0 0.0 null null null null)
  (`KismetSystemLibrary.Delay` (`PaperFlipbookComponent.GetFlipbookLength` (`self.Explosion Flipbook`)))
  (`self.K2_DestroyActor`))

(event `self.Explosion Splash Collision.OnComponentBeginOverlap`
  (params (OverlappedComponent :type "PrimitiveComponent Object Reference") (OtherActor :type "Actor Object Reference") (OtherComp :type "PrimitiveComponent Object Reference") (OtherBodyIndex :type Integer) (bFromSweep :type Boolean) (SweepResult :type "HitResult Structure (by ref)"))
  (bind _asbp_enemy (cast `/Game/DirtyManners/Blueprints/Enemies/BP_Enemy` OtherActor))
  (bind _returnvalue (`AbilitySystemBlueprintLibrary.GetAbilitySystemComponent` _asbp_enemy))
  (`AbilitySystemComponent.BP_ApplyGameplayEffectToTarget` _returnvalue "/Game/DirtyManners/Blueprints/Abilities/Launcher/GE_PlayerLauncherExplosionDamage.GE_PlayerLauncherExplosionDamage_C" _returnvalue 0.0 (`AbilitySystemComponent.MakeEffectContext` _returnvalue))
  (bind _asbp_fpsplayer (cast `/Game/DirtyManners/Blueprints/Player/BP_FPSPlayer` (`GameplayStatics.GetPlayerPawn` 0)))
  (`/Game/DirtyManners/Blueprints/Widgets/WBP_Hud.Increase Points` (`/Game/DirtyManners/Blueprints/Player/BP_FPSPlayer.HUD` _asbp_fpsplayer) 5))

(fn `UserConstructionScript`)