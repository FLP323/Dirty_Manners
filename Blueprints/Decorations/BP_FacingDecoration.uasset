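; Decoration actor that shows a configurable paper sprite which always turns to face the player camera, like a billboard.
; BeginPlay assigns DecorationSprite to the Sprite component.
; Every Tick it yaws the sprite toward the camera location with a 90-degree offset, keeping pitch and roll at zero so it stays upright.
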(event `self.ReceiveBeginPlay`
  (`PaperSpriteComponent.SetSprite` (`self.Sprite`) (`self.DecorationSprite`)))

(event `self.ReceiveTick`
  (params (DeltaSeconds :type "Float (single-precision)"))
  (bind _returnvalue (`GameplayStatics.GetPlayerCameraManager` 0))
  (bind _sprite (`self.Sprite`))
  (bind (_returnvalue_roll _returnvalue_pitch _returnvalue_yaw) (`KismetMathLibrary.BreakRotator` (`KismetMathLibrary.FindLookAtRotation` (`SceneComponent.K2_GetComponentLocation` _sprite) (`PlayerCameraManager.GetCameraLocation` _returnvalue))))
  (`/Engine/EditorBlueprintResources/StandardMacros.IsValid` _returnvalue
    (:`Is Valid`
      (`SceneComponent.K2_SetWorldRotation` _sprite (`KismetMathLibrary.MakeRotator` 0.0 0.0 (- _returnvalue_yaw 90.0)) false false))))

(fn `UserConstructionScript`)