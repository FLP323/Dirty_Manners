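; Respawning weapon pickup that grants a Water Gun, Launcher or Bubbler, shown as a Paper2D flipbook chosen by WeaponToAcquire at construction.
; On overlap, it compares player 0's ability-system attribute against that weapon's max bullets, rockets or soap.
; If below max, it calls WeaponPickup on the overlapping BP_FPSPlayer and plays a sound.
; It then clears the sprite and stays inactive for a fixed cooldown before restoring it.
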(event `self.ReceiveActorBeginOverlap`
  (params (OtherActor :type "Actor Object Reference"))
  (bind _returnvalue (`GameplayStatics.GetPlayerPawn` 0))
  (bind _returnvalue_2 (`GameplayStatics.GetPlayerPawn` 0))
  (bind _returnvalue_3 (`GameplayStatics.GetPlayerPawn` 0))
  (if (not (`self.Cooldown`))
    (switch `/Game/DirtyManners/Blueprints/Enums/ENUM_WeaponList` (`self.Weapon To Acquire`)
      (:`NewEnumerator0`
        (bind _asbp_dirty_manners_character (cast `/Game/DirtyManners/Blueprints/BP_DirtyMannersCharacter` _returnvalue_2))
        (if (not (>= (`.ReturnValue` (`AbilitySystemBlueprintLibrary.GetFloatAttributeFromAbilitySystemComponent` (`AbilitySystemBlueprintLibrary.GetAbilitySystemComponent` _returnvalue_2) (struct :`AttributeName` "Bullets" :`Attribute` "/Script/Dirty_Manners.DirtyMannersAttributeSet:Bullets" :`AttributeOwner` "/Script/CoreUObject.Class'/Script/Dirty_Manners.DirtyMannersAttributeSet'"))) (`DirtyMannersCharacter.MaxBullets` _asbp_dirty_manners_character)))
          (bind _asbp_fpsplayer (cast `/Game/DirtyManners/Blueprints/Player/BP_FPSPlayer` OtherActor :!label _label))
          (`/Game/DirtyManners/Blueprints/Player/BP_FPSPlayer.Weapon Pickup` _asbp_fpsplayer (`self.Weapon To Acquire`))
          (`GameplayStatics.PlaySoundAtLocation` "/Game/DirtyManners/SFX/ItemPickup_SFX.ItemPickup_SFX" (`SceneComponent.K2_GetComponentLocation` (`self.DefaultSceneRoot`)) (struct) 0.5 1.0 0.0 null null null null)
          (`PaperFlipbookComponent.SetFlipbook` (`self.Item Sprite`) null)
          (set `self.Cooldown` true)
          (`KismetSystemLibrary.Delay` 15.0)
          (`self.Set Flipbook`)
          (set `self.Cooldown` false)))
      (:`NewEnumerator1`
        (bind _asbp_dirty_manners_character_2 (cast `/Game/DirtyManners/Blueprints/BP_DirtyMannersCharacter` _returnvalue))
        (if (not (>= (`.ReturnValue` (`AbilitySystemBlueprintLibrary.GetFloatAttributeFromAbilitySystemComponent` (`AbilitySystemBlueprintLibrary.GetAbilitySystemComponent` _returnvalue) (struct :`AttributeName` "Rockets" :`Attribute` "/Script/Dirty_Manners.DirtyMannersAttributeSet:Rockets" :`AttributeOwner` "/Script/CoreUObject.Class'/Script/Dirty_Manners.DirtyMannersAttributeSet'"))) (`DirtyMannersCharacter.MaxRockets` _asbp_dirty_manners_character_2)))
          (goto _label)))
      (:`NewEnumerator3`
        (bind _asbp_dirty_manners_character_3 (cast `/Game/DirtyManners/Blueprints/BP_DirtyMannersCharacter` _returnvalue_3))
        (if (not (>= (`.ReturnValue` (`AbilitySystemBlueprintLibrary.GetFloatAttributeFromAbilitySystemComponent` (`AbilitySystemBlueprintLibrary.GetAbilitySystemComponent` _returnvalue_3) (struct :`AttributeName` "Soap" :`Attribute` "/Script/Dirty_Manners.DirtyMannersAttributeSet:Soap" :`AttributeOwner` "/Script/CoreUObject.Class'/Script/Dirty_Manners.DirtyMannersAttributeSet'"))) (`DirtyMannersCharacter.MaxSoap` _asbp_dirty_manners_character_3)))
          (goto _label))))))

(fn `Set Flipbook`
  (bind _item_sprite (`self.Item Sprite`))
  (switch `/Game/DirtyManners/Blueprints/Enums/ENUM_WeaponList` (`self.Weapon To Acquire`)
    (:`NewEnumerator2`
      (`PaperFlipbookComponent.SetFlipbook` _item_sprite null))
    (:`NewEnumerator0`
      (`PaperFlipbookComponent.SetFlipbook` _item_sprite "/Game/DirtyManners/Flipbooks/Pickups/FB_PistolPickup.FB_PistolPickup"))
    (:`NewEnumerator1`
      (`PaperFlipbookComponent.SetFlipbook` _item_sprite "/Game/DirtyManners/Flipbooks/Launcher/FB_Launcher_Pickup.FB_Launcher_Pickup"))
    (:`NewEnumerator3`
      (`PaperFlipbookComponent.SetFlipbook` _item_sprite "/Game/DirtyManners/Flipbooks/Bubbler/FB_Bubbler_Pickup.FB_Bubbler_Pickup"))))

(fn `UserConstructionScript`
  (`self.Set Flipbook`))