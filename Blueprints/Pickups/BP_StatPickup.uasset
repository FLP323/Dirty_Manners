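; Paper2D stat pickup that comes as health or armor, in small or large size.
; Construction calls the parent script, then sets the flipbook, sprite scale and pickup gameplay tag from type and size.
; Separate health and armor checks read an Ability System attribute and add a Player Full tag to the pickup's tags at exactly 100, removing it otherwise.
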(fn `Full Armor  Check`
  (params (`Ability System` :type "AbilitySystemComponent Object Reference"))
  (bind _pickup_tag (`self.Pickup Tag`))
  (if (== (`.ReturnValue` (`AbilitySystemBlueprintLibrary.GetFloatAttributeFromAbilitySystemComponent` `Ability System` (struct :`AttributeName` "Armor" :`Attribute` "/Script/Dirty_Manners.DirtyMannersAttributeSet:Armor" :`AttributeOwner` "/Script/CoreUObject.Class'/Script/Dirty_Manners.DirtyMannersAttributeSet'"))) 100.0)
    (`BlueprintGameplayTagLibrary.AddGameplayTag` _pickup_tag (struct :`TagName` "Player.Armor.Full"))
    (else
      (`BlueprintGameplayTagLibrary.RemoveGameplayTag` _pickup_tag (struct :`TagName` "Player.Armor.Full")))))

(fn `Full Health Check`
  (params (`Ability System` :type "AbilitySystemComponent Object Reference"))
  (bind _pickup_tag (`self.Pickup Tag`))
  (if (== (`.ReturnValue` (`AbilitySystemBlueprintLibrary.GetFloatAttributeFromAbilitySystemComponent` `Ability System` (struct :`AttributeName` "Health" :`Attribute` "/Script/Dirty_Manners.DirtyMannersAttributeSet:Health" :`AttributeOwner` "/Script/CoreUObject.Class'/Script/Dirty_Manners.DirtyMannersAttributeSet'"))) 100.0)
    (`BlueprintGameplayTagLibrary.AddGameplayTag` _pickup_tag (struct :`TagName` "Player.Health.Full"))
    (else
      (`BlueprintGameplayTagLibrary.RemoveGameplayTag` _pickup_tag (struct :`TagName` "Player.Health.Full")))))

(fn `Set Stat Pickup Flipbook`
  (bind _item_sprite (`self.Item Sprite`))
  (bind _item_sprite_2 (`self.Item Sprite`))
  (switch `/Game/DirtyManners/Blueprints/Enums/ENUM_PickupType` (`self.Pickup Type`)
    (:`NewEnumerator0`
      (`PaperFlipbookComponent.SetFlipbook` _item_sprite "/Game/DirtyManners/Flipbooks/Pickups/FB_ArmorPickup.FB_ArmorPickup")
      (switch `/Game/DirtyManners/Blueprints/Enums/ENUM_PickupSize` (`self.Pickup Size`)
        (:`NewEnumerator0`
          (`SceneComponent.SetRelativeScale3D` _item_sprite_2 (1.0 1.0 1.0))
          (set `self.Pickup Tag` (struct :`GameplayTags` (struct :`(TagName` "Pickup.Armor.Small")))))
        (:`NewEnumerator1`
          (`SceneComponent.SetRelativeScale3D` _item_sprite_2 (2.0 2.0 2.0))
          (set `self.Pickup Tag` (struct :`GameplayTags` (struct :`(TagName` "Pickup.Armor.Large")))))))
    (:`NewEnumerator1`
      (`PaperFlipbookComponent.SetFlipbook` _item_sprite "/Game/DirtyManners/Flipbooks/Pickups/FB_HealthPickup.FB_HealthPickup")
      (switch `/Game/DirtyManners/Blueprints/Enums/ENUM_PickupSize` (`self.Pickup Size`)
        (:`NewEnumerator0`
          (`SceneComponent.SetRelativeScale3D` _item_sprite_2 (1.0 1.0 1.0))
          (set `self.Pickup Tag` (struct :`GameplayTags` (struct :`(TagName` "Pickup.Health.Small")))))
        (:`NewEnumerator1`
          (`SceneComponent.SetRelativeScale3D` _item_sprite_2 (2.0 2.0 2.0))
          (set `self.Pickup Tag` (struct :`GameplayTags` (struct :`(TagName` "Pickup.Health.Large")))))))))

(fn `UserConstructionScript`
  (`parent.UserConstructionScript`)
  (`self.Set Stat Pickup Flipbook`))