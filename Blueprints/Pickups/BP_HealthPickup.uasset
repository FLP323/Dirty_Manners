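; Health pickup with a flipbook sprite that triggers a Gameplay Ability System ability on the overlapping BP_FPSPlayer and respawns after a cooldown.
; On overlap it runs FullHealthCheck on the player's ability system, then tries to activate abilities by PickupTag.
; Success notifies the player, plays a sound, clears the sprite and blocks reuse during a delay.
; It then calls the parent construction script to reset itself.
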(event `self.ReceiveActorBeginOverlap`
  (params (OtherActor :type "Actor Object Reference"))
  (if (not (`self.Cooldown`))
    (bind _asbp_fpsplayer (cast `/Game/DirtyManners/Blueprints/Player/BP_FPSPlayer` OtherActor))
    (bind _abilitysystemcomponent (`DirtyMannersCharacter.AbilitySystemComponent` _asbp_fpsplayer))
    (`self.Full Health Check` _abilitysystemcomponent)
    (bind _returnvalue (`AbilitySystemComponent.TryActivateAbilitiesByTag` _abilitysystemcomponent (`self.Pickup Tag`) false))
    (if _returnvalue
      (`/Game/DirtyManners/Blueprints/Player/BP_FPSPlayer.Item Pickup` _asbp_fpsplayer)
      (`GameplayStatics.PlaySoundAtLocation` "/Game/DirtyManners/SFX/Health_SFX.Health_SFX" (`SceneComponent.K2_GetComponentLocation` (`self.DefaultSceneRoot`)) (struct) 0.3 1.0 0.0 null null null null)
      (set `self.Cooldown` true)
      (`PaperFlipbookComponent.SetFlipbook` (`self.Item Sprite`) null)
      (`KismetSystemLibrary.Delay` 20.0)
      (`parent.UserConstructionScript`)
      (set `self.Cooldown` false))))

(fn `UserConstructionScript`
  (`parent.UserConstructionScript`))